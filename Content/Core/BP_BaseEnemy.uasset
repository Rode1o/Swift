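; BP_BaseEnemy is an enemy base Blueprint that displays the enemy's awareness state through a Status text render component.
; SetEnemyStatus takes the new state and selects both the symbol and its color: blank for Patrol, "?" in SearchingColor for Searching, "!" in ChasingColor for Alert.
; It holds no detection or movement logic, and its construction script is empty.
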(event `self.BP_SetEnemyStatus`
  (params (NewEnemyStatus :type "E_EnemyStatus Enum" :default "EnemyStatus_Patrol"))
  (`TextRenderComponent.K2_SetText` (`self.Status`) (select `E_EnemyStatus` NewEnemyStatus :`EnemyStatus_Patrol` "" :`EnemyStatus_Searching` "?" :`EnemyStatus_Alert` "!"))
  (`TextRenderComponent.SetTextRenderColor` (`self.Status`) (select `E_EnemyStatus` NewEnemyStatus :`EnemyStatus_Searching` (`self.SearchingColor`) :`EnemyStatus_Alert` (`self.ChasingColor`))))

(fn `UserConstructionScript`)