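; Player character Blueprint that shows a stamina widget on begin play and handles takedowns of enemies.
; When CanTakedown is set, pressing Attack reports a noise at the player and finds the nearest BP_BaseEnemy.
; That enemy gets its material swapped and its mesh set to simulate physics, then a shutdown sound plays and the flag clears.
; The flag is not set to true anywhere in this graph.
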(event `self.ReceiveBeginPlay`
  (bind _returnvalue (`|CreateWidget` "/Game/Core/WDG_Stamina.WDG_Stamina_C"))
  (`UserWidget.AddToViewport` _returnvalue 0))

(event `InputAction|Attack`
  (params (Key :type "Key Structure"))
  (bind _returnvalue (`self.K2_GetActorLocation` (`GameplayStatics.GetPlayerCharacter` 0)))
  (:`Pressed`
    (if (`self.CanTakedown`)
      (`AISense_Hearing.ReportNoiseEvent` _returnvalue 2.0 self 1000.0)
      (bind (_nearestlocation _nearestactor) (`/Game/Core/BP_FunctionNearest.NearestEnemy` "/Game/Core/BP_BaseEnemy.BP_BaseEnemy_C" _returnvalue))
      (bind _asbp_base_enemy (cast `/Game/Core/BP_BaseEnemy` _nearestactor))
      (bind _mesh (`Character.Mesh` _asbp_base_enemy))
      (`PrimitiveComponent.SetMaterial` _mesh 0 "/Game/StarterContent/Materials/M_Basic_Wall.M_Basic_Wall")
      (`PrimitiveComponent.SetSimulatePhysics` _mesh true)
      (`GameplayStatics.PlaySound2D` "/Game/Core/ShutDown.ShutDown" 1.0 1.0 0.0 null null)
      (set `self.CanTakedown` false))))

(fn `UserConstructionScript`)